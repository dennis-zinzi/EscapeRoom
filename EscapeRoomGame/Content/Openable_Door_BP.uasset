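; Door actor Blueprint that swings open and closed when its OpenDoor component fires open and close events.
; The DoorSwing timeline plays on open and reverses on close, scaling its curve by the component's OpenAngle to set yaw relative to the rotation captured at BeginPlay.
; An event track on the timeline times the door lock sound at the door's location.
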(event `self.ReceiveBeginPlay`
  (set `self.Start Rotation` (`self.K2_GetActorRotation`)))

(event `self.OpenDoor.OnOpenDoor`
  (bind (_direction _openangle) (`Timeline|Door Swing` :!label _label)
    (:`Update`
      (`self.K2_SetActorRotation` (`KismetMathLibrary.ComposeRotators` (`self.Start Rotation`) (`KismetMathLibrary.MakeRotator` 0.0 0.0 (* _openangle (`OpenDoor.OpenAngle` (`self.OpenDoor`)))))))
    (:`Sound Timing`
      (`GameplayStatics.PlaySoundAtLocation` "/Game/Audio/door-lock.door-lock" (`self.K2_GetActorLocation`)))))

(event `self.OpenDoor.OnCloseDoor`
  (goto _label :!via `Reverse`))

(fn `UserConstructionScript`)